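; Pickup item Blueprint that hands the player tools and prompts them to head to the farm.
; On box overlap, it fetches player 0's character, not the overlapping actor, and snaps the Item component to a socket on that character.
; It then shows the message through DemoHud's DrawTextToScreen.
; Ending the actor overlap reuses the same HUD call with empty text to clear the message.
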(event OnComponentBeginOverlap(Box)
  (params (OverlappedComponent :type Primitive%20Component%20Object%20Reference) (OtherActor :type Actor%20Object%20Reference) (OtherComp :type Primitive%20Component%20Object%20Reference) (OtherBodyIndex :type Integer) (bFromSweep :type Boolean) (SweepResult :type Hit%20Result%20Structure%20%28by%20ref%29))
  (bind _asthird_person_demo_character (Utilities|Casting|CastToThirdPersonDemoCharacter (Game|GetPlayerCharacter 0)))
  (Transformation|AttachComponentToComponent (Variables|Default|GetItem) (Variables|/Game/Assets/Blueprints/ThirdPersonDemoCharacter.ThirdPersonDemoCharacter_C|GetNewVar_1 _asthird_person_demo_character) "Socket" "SnapToTarget" "SnapToTarget" "SnapToTarget" true)
  (Variables|Default|SetText "Tools obtained! Head to the farm!")
  (bind _asdemo_hud (Utilities|Casting|CastToDemoHud (HUD|GetHUD (Game|GetPlayerController 0))))
  (Default|DrawTexttoScreen _asdemo_hud true (Variables|Default|GetText)))

(event Collision|EventActorEndOverlap
  (params (OtherActor :type Actor%20Object%20Reference))
  (Variables|Default|SetText "")
  (bind _asdemo_hud (Utilities|Casting|CastToDemoHud (HUD|GetHUD (Game|GetPlayerController 0))))
  (Default|DrawTexttoScreen _asdemo_hud true (Variables|Default|GetText)))

(fn ConstructionScript)