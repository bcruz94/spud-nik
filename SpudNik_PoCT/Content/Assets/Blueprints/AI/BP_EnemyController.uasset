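; Enemy AI controller that runs the BT_Enemy behavior tree on possession and feeds it perception results through the Blackboard.
; When perception senses a player-controlled Character, it sets CanSeePlayer true and stores that actor as TargetActor.
; Any other Character update, including losing the player, sets CanSeePlayer false but leaves TargetActor in place.
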(event OnTargetPerceptionUpdated(AIPerception)
  (params (Actor :type Actor%20Object%20Reference) (Stimulus :type AI%20Stimulus%20Structure))
  (bind _blackboard (Variables|Default|GetBlackboard))
  (bind _ascharacter (Utilities|Casting|CastToCharacter Actor))
  (if (and (Pawn|IsPlayerControlled _ascharacter) (Utilities|Struct|BreakAIStimulus Stimulus))
    (AI|Components|Blackboard|SetValueasBool _blackboard (Utilities|Name|MakeLiteralName "CanSeePlayer") true)
    (AI|Components|Blackboard|SetValueasObject _blackboard (Utilities|Name|MakeLiteralName "TargetActor") Actor)
    (else
      (AI|Components|Blackboard|SetValueasBool _blackboard (Utilities|Name|MakeLiteralName "CanSeePlayer") false))))

(event EventBeginPlay)

(event EventTick
  (params (DeltaSeconds :type Float%20%28single-precision%29)))

(event EventPossess
  (params (PossessedPawn :type Pawn%20Object%20Reference))
  (AI|RunBehaviorTree "/Game/Assets/Blueprints/AI/BT_Enemy.BT_Enemy"))

(fn ConstructionScript)