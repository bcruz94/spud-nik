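; TechPrototypeDemo runs a countdown game timer that prints "Game Over" and pauses the game at zero.
; BeginPlay loads minutes and seconds from GameTimeInstance and adds the Timer widget to the viewport.
; Tick uses a Delay to count down once per second, rolling seconds into minutes.
; It writes the time back to the game instance, except when seconds equal zero.
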(event EventBeginPlay
  ;[1 1 1] Viewmode Unlit/Timer On Screen
  (bind _asgame_time_instance (Utilities|Casting|CastToGameTimeInstance (Game|GetGameInstance)))
  (Variables|Default|SetTimeMin (Variables|/Game/Blueprints/GameTimeInstance.GameTimeInstance_C|GetTimeMin _asgame_time_instance))
  (Variables|Default|SetTimeSec (Variables|/Game/Blueprints/GameTimeInstance.GameTimeInstance_C|GetTimeSec _asgame_time_instance))
  (bind _returnvalue (UserInterface|CreateWidget "/Game/Assets/Blueprints/Timer.Timer_C"))
  (UserInterface|Viewport|AddtoViewport _returnvalue 0))

(event EventTick
  (params (DeltaSeconds :type Float%20%28single-precision%29))
  ;[1 1 1] Game Timer
  (Utilities|FlowControl|Delay 1.0)
  (Variables|Default|SetTimeSec (- (Variables|Default|GetTimeSec) 1))
  (if (< (Variables|Default|GetTimeSec) 0)
    (Variables|Default|SetTimeMin (- (Variables|Default|GetTimeMin) 1))
    (Variables|Default|SetTimeSec 59))
  (if (== (Variables|Default|GetTimeSec) 0)
    (if (== (Variables|Default|GetTimeMin) 0)
      (Development|PrintString "Game Over")
      (Game|SetGamePaused true))
    (else
      (bind _asgame_time_instance (Utilities|Casting|CastToGameTimeInstance (Game|GetGameInstance)))
      (Variables|/Game/Blueprints/GameTimeInstance.GameTimeInstance_C|SetTimeSec _asgame_time_instance (Variables|Default|GetTimeSec))
      (Variables|/Game/Blueprints/GameTimeInstance.GameTimeInstance_C|SetTimeMin _asgame_time_instance (Variables|Default|GetTimeMin)))))

(fn ConstructionScript)