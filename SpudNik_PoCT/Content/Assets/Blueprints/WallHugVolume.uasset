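; Trigger volume that marks where the third-person demo character can hug a wall.
; When that character enters the Box, it calls TurnOnHug with the Direction component's forward vector as the axis and the world locations of LeftEdge and RightEdge.
; Leaving the Box calls TurnOffHug, and both events print an on-screen debug message.
; The hug behavior itself lives in the character; the volume only supplies the geometry.
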(event OnComponentBeginOverlap(Box)
  (params (OverlappedComponent :type Primitive%20Component%20Object%20Reference) (OtherActor :type Actor%20Object%20Reference) (OtherComp :type Primitive%20Component%20Object%20Reference) (OtherBodyIndex :type Integer) (bFromSweep :type Boolean) (SweepResult :type Hit%20Result%20Structure%20%28by%20ref%29))
  (bind _asthird_person_demo_character (Utilities|Casting|CastToThirdPersonDemoCharacter OtherActor))
  (Default|TurnonHug _asthird_person_demo_character (Math|Vector|GetForwardVector (Variables|Default|GetDirection)) (Transformation|GetWorldLocation (Variables|Default|GetLeftEdge)) (Transformation|GetWorldLocation (Variables|Default|GetRightEdge)))
  (Development|PrintString "Can Hug!!" true false))

(event OnComponentEndOverlap(Box)
  (params (OverlappedComponent :type Primitive%20Component%20Object%20Reference) (OtherActor :type Actor%20Object%20Reference) (OtherComp :type Primitive%20Component%20Object%20Reference) (OtherBodyIndex :type Integer))
  (bind _asthird_person_demo_character (Utilities|Casting|CastToThirdPersonDemoCharacter OtherActor))
  (Default|TurnOffHug _asthird_person_demo_character)
  (Development|PrintString "Can't Hug" true false))

(event EventBeginPlay)

(event Collision|EventActorBeginOverlap
  (params (OtherActor :type Actor%20Object%20Reference)))

(event EventTick
  (params (DeltaSeconds :type Float%20%28single-precision%29)))

(fn ConstructionScript)