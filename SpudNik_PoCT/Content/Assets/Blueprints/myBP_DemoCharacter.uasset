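; Demo character Blueprint that handles the player side of key-press quick time events.
; BeginPlay adds the main widget to the viewport and sets game-only input.
; Any key press resolves a pending event as success or wrong-key failure by comparing it to the expected key.
; On completion it resets time dilation, blends the camera back to itself if one was switched, and plays the result animation before removing the event widget.
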(event Custom|OnEventCompleted
  (params (Result :type e_EventState%20Enum :default "NewEnumerator0") (CameraTransition :type S%20Camera%20Transition%20Structure))
  (bind (_newcamera _blendtime) (Utilities|Struct|Breaks_CameraTransition CameraTransition))
  (Variables|Default|SetCustomTimeDilation 1.0)
  (Utilities|IsValid _newcamera
    (:Is%20Valid
      (Game|Player|SetViewTargetwithBlend (Game|GetPlayerController 0) self _blendtime "VTBlend_Linear" 0.0 false))
    (:Is%20Not%20Valid
      _))
  (Utilities|IsValid (Variables|Default|GetEventWidget)
    (:Is%20Valid
      (UserInterface|Animation|PlayAnimation (Variables|Default|GetEventWidget) (select (Utilities|Enum|Equal(Enum) Result "NewEnumerator2") (Variables|/Game/QuickTime/W_QuickTimeEvent.W_QuickTimeEvent_C|GetSuccess (Variables|Default|GetEventWidget)) (Variables|/Game/QuickTime/W_QuickTimeEvent.W_QuickTimeEvent_C|GetFailure (Variables|Default|GetEventWidget))) 0.0 1 "Forward" 1.0)
      (Utilities|FlowControl|Delay (Class|WidgetAnimation|GetEndTime (select (Utilities|Enum|Equal(Enum) Result "NewEnumerator2") (Variables|/Game/QuickTime/W_QuickTimeEvent.W_QuickTimeEvent_C|GetSuccess (Variables|Default|GetEventWidget)) (Variables|/Game/QuickTime/W_QuickTimeEvent.W_QuickTimeEvent_C|GetFailure (Variables|Default|GetEventWidget)))))
      (Widget|RemovefromParent (Variables|Default|GetEventWidget))
      (Variables|Default|SetEventWidget 0))))

(event EventBeginPlay
  (bind _returnvalue (UserInterface|CreateWidget "/Game/QuickTime/W_Main.W_Main_C"))
  (Variables|Default|SetMainWidget _returnvalue)
  (Input|SetInputModeGameOnly (Game|GetPlayerController 0))
  (UserInterface|Viewport|AddtoViewport (Variables|Default|GetMainWidget) 0))

(event Input|KeyboardEvents|AnyKey
  (params (Key :type Key%20Structure))
  (bind _currentevent (Variables|Default|GetCurrentEvent))
  (bind (_state _key) (Utilities|Struct|Breaks_EventInfo _currentevent))
  (:Pressed
    (switch Utilities|FlowControl|Switch|Switchone_EventState _state
      (:NewEnumerator1
        (if (== _key Key)
          (Utilities|Struct|Setmembersins_EventInfo (Variables|Default|GetCurrentEvent) "NewEnumerator2")
          (else
            (Utilities|Struct|Setmembersins_EventInfo (Variables|Default|GetCurrentEvent) "NewEnumerator4")))))))

(fn ConstructionScript)